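; BP_Cube is an actor that moves vertically around its starting position, driven by a float curve.
; BeginPlay stores the origin location, and Tick accumulates elapsed time to sample the curve.
; The curve value, scaled to a height offset, is added to the origin and applied without sweep.
; Time is never wrapped in the graph, so any repetition depends on the curve itself.
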(event `self.ReceiveBeginPlay`
  (set `self.OriginLocation` (`self.K2_GetActorLocation`)))

(event `self.ReceiveTick`
  (params (DeltaSeconds :type "Float (single-precision)"))
  (set `self.CurTime` (+ (`self.CurTime`) DeltaSeconds))
  (`self.K2_SetActorLocation` (+ (`self.OriginLocation`) (`KismetMathLibrary.MakeVector` 0.0 0.0 (* (`CurveFloat.GetFloatValue` (`self.Curve`) (`self.CurTime`)) 100.0)))))

(fn `UserConstructionScript`)