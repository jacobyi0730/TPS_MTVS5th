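; Test enemy AI for the TPS game that patrols waypoints and chases the player, using a two-state switch evaluated on Tick.
; BeginPlay gathers StaticMeshActors tagged WayPoint and picks a random starting one.
; Patrol reissues AIMoveTo each frame, cycles waypoints behind a delay-reset DoOnce, and sphere-checks for BP_TPSPlayer.
; Detection switches to Chase, which follows that player with no return to Patrol.
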(event `self.ReceiveBeginPlay`
  (`|ExecutionSequence`
    (:`then_0`
      (bind _outactors (`GameplayStatics.GetAllActorsOfClassWithTag` "/Script/Engine.StaticMeshActor" "WayPoint"))
      (set `self.Path` _outactors))
    (:`then_1`
      (set `self.Index` (`KismetMathLibrary.RandomIntegerInRange` 0 (`KismetArrayLibrary.Array_LastIndex` (`self.Path`)))))
    (:`then_2`
      (set `self.Target` (`|GetArrayItem` (`self.Path`) (`self.Index`))))
    (:`then_3`
      (set `self.State` "NewEnumerator0"))))

(event `self.ReceiveTick`
  (params (DeltaSeconds :type "Float (single-precision)"))
  (switch `/Game/TPS/Blueprints/AI/ETestEnemyState` (`self.State`)
    (:`NewEnumerator0`
      (`|ExecutionSequence`
        (:`then_0`
          (`|AIMoveTo` self (0.0 0.0 0.0) (`self.Target`) 150.0
            (:`OnSuccess`
              (`/Engine/EditorBlueprintResources/StandardMacros.DoOnce` false :!label _label
                (:`Completed`
                  (bind _result (`/Engine/EditorBlueprintResources/StandardMacros.IncrementInt` (`self.Index`))
                    (:`  `
                      (set `self.Index` (mod _result (`KismetArrayLibrary.Array_Length` (`self.Path`))))
                      (set `self.Target` (`|GetArrayItem` (`self.Path`) (`self.Index`)))
                      (`KismetSystemLibrary.Delay` 0.2)
                      (goto _label :!via `Reset`))))))))
        (:`then_1`
          (bind (_outactors _returnvalue) (`KismetSystemLibrary.SphereOverlapActors` (`self.K2_GetActorLocation`) 500.0 (`|MakeArray` "ObjectTypeQuery3" :!type "EObjectTypeQuery Enum") "/Game/TPS/Blueprints/BP_TPSPlayer.BP_TPSPlayer_C" (`|MakeArray` self :!type "Actor Object Reference")))
          (if _returnvalue
            (set `self.ChaseTarget` (`|GetArrayItem` _outactors))
            (set `self.State` "NewEnumerator1")))))
    (:`NewEnumerator1`
      (`|AIMoveTo` self (0.0 0.0 0.0) (`self.ChaseTarget`) 150.0))))

(fn `UserConstructionScript`)